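; Paper2D ghost enemy that kills the player character on overlap while active.
; After a startup delay, Tick keeps a timeline playing that moves it by a scaled vector offset from its spawn location.
; Overlapping a WindActor makes it invisible and harmless for a set delay, then restores it through the shared Desactivation function, while movement continues.
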(event `self.ReceiveBeginPlay`
  (set `self.locghost` (`self.K2_GetActorLocation`))
  (`KismetSystemLibrary.Delay` (`self.startghost`))
  (set `self.start` true))

(event `self.ReceiveActorBeginOverlap`
  (params (OtherActor :type "Actor Object Reference"))
  (if (`self.active`)
    (bind _aspaper_charactertest (cast `/Game/Blueprints/PaperCharactertest` OtherActor)
      (:`then`
        (`/Game/Blueprints/PaperCharactertest.deathplayer` _aspaper_charactertest))
      (:`CastFailed`
        (cast `/Game/Blueprints/WindActor` OtherActor)
        (`self.desactivation` false)
        (`KismetSystemLibrary.Delay` (`self.delaydeactivate`))
        (`self.desactivation` true)))))

(event `self.ReceiveTick`
  (params (DeltaSeconds :type "Float (single-precision)"))
  (if (`self.start`)
    (`|ExecutionSequence`
      (:`then_0`
        (bind (_direction _ghostvectorx) (`Timeline|ghosttimeline`)
          (:`Update`
            (`self.K2_SetActorLocation` (+ (* _ghostvectorx (`self.coef`)) (`self.locghost`)))))))))

(fn `desactivation`
  (params (bool :type Boolean))
  (set `self.active` bool)
  (`SceneComponent.SetVisibility` (`self.PaperSprite`) bool false))

(fn `UserConstructionScript`)