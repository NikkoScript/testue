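; SpriteLever is a lever actor that switches on when any actor overlaps it and switches itself off after a countdown.
; On BeginPlay it creates a Statelever widget, passes itself as the Lever reference and adds it to the viewport.
; Overlap sets Activated and restarts a Delay counter, which Tick decrements each frame, clearing Activated at zero, so the active time depends on frame rate.
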(event `self.ReceiveBeginPlay`
  (bind _returnvalue (`|CreateWidget` "/Game/Blueprints/statelever.statelever_C"))
  (set `/Game/Blueprints/statelever.Lever` self _returnvalue)
  (`UserWidget.AddToViewport` _returnvalue 0))

(event `self.ReceiveActorBeginOverlap`
  (params (OtherActor :type "Actor Object Reference"))
  (`KismetSystemLibrary.PrintString` "windactor")
  (set `self.Activated` true)
  (set `self.delay` 100))

(event `self.ReceiveTick`
  (params (DeltaSeconds :type "Float (single-precision)"))
  (bind _delay (`self.delay`))
  (`/Engine/EditorBlueprintResources/StandardMacros.DecrementInt` _delay
    (:`  `
      (if (== (`KismetMathLibrary.Conv_IntToDouble` _delay) 0.0)
        (set `self.Activated` false)))))

(fn `UserConstructionScript`)