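; PaperCharactertest is a 2D side-scrolling player character with flipbook animation, jumping, climbing and a chargeable wind ability.
; A state enum gates running, jumping and climbing; climbing disables movement mode and sweeps the actor vertically.
; Tick swaps idle/run flipbooks, flips facing through control rotation and refills the charge spent spawning a directional WindActor.
; Death respawns and possesses a fresh copy at the start transform; death and Use are broadcast through Call events.
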(event `deathplayer`
  (`KismetSystemLibrary.PrintString` "death")
  (`self.K2_DestroyActor` (`GameplayStatics.GetPlayerCharacter` 0))
  (bind _returnvalue (`|SpawnActorFromClass` "PaperCharactertest_C" (`self.startlocation`) "Undefined" "OverrideRootScale" null null))
  (`Controller.Possess` (`GameplayStatics.GetPlayerController` 0) _returnvalue)
  (`self.death`))

(event `InputAxis|MoveRight`
  (params (AxisValue :type "Float (single-precision)"))
  (switch `/Game/Blueprints/use/echelle/PlayerDefinedEnume` (`self.PlayerEnume`)
    (:`NewEnumerator0`
      (`self.AddMovementInput` (* (1.0 0.0 0.0) AxisValue)))))

(event `self.ReceiveTick`
  (params (DeltaSeconds :type "Float (single-precision)"))
  (bind _returnvalue (`self.GetController`))
  (bind _returnvalue_x (`KismetMathLibrary.BreakVector` (`self.GetVelocity`)))
  (bind _windcharge (`self.windcharge`))
  (if (< _windcharge 100.0)
    (`/Engine/EditorBlueprintResources/StandardMacros.IncrementFloat` _windcharge
      (:`  `
        _)))
  (`|ExecutionSequence`
    (:`then_0`
      (if (> (`KismetMathLibrary.VSize` (`self.GetVelocity`)) 0.0)
        (`PaperFlipbookComponent.SetFlipbook` (`self.Sprite`) "/Game/2DSideScroller/Textures/runanim.runanim")
        (set `self.running` true)
        (set `self.idle` false)
        (else
          (`PaperFlipbookComponent.SetFlipbook` (`self.Sprite`) "/Game/2DSideScroller/Textures/idle.idle")
          (set `self.running` false)
          (set `self.idle` true))))
    (:`then_1`
      (if (`self.running`)
        (if (> _returnvalue_x 0.0)
          (`Controller.SetControlRotation` _returnvalue (`KismetMathLibrary.MakeRotator` 0.0))
          (else
            (`Controller.SetControlRotation` _returnvalue (`KismetMathLibrary.MakeRotator` 0.0 0.0 180.0))))))))

(event `InputAction|Jump`
  (params (Key :type "Key Structure"))
  (bind _playerenume (`self.PlayerEnume`))
  (:`Pressed`
    (switch `/Game/Blueprints/use/echelle/PlayerDefinedEnume` _playerenume
      (:`NewEnumerator0`
        (`self.Jump`)
        (`KismetSystemLibrary.PrintString` (`|GetEnumeratorNameAsString` _playerenume))))))

(event `InputAction|Wind`
  (params (Key :type "Key Structure"))
  (bind _returnvalue_x (`KismetMathLibrary.BreakVector` (`self.GetActorForwardVector`)))
  (bind _returnvalue (`KismetMathLibrary.SignOfFloat` _returnvalue_x))
  (:`Pressed`
    (if (== (`self.windcharge`) 100.0)
      (bind _returnvalue_2 (`|SpawnActorFromClass` "/Game/Blueprints/WindActor.WindActor_C" (`KismetMathLibrary.MakeTransform` (`self.K2_GetActorLocation`) (`self.K2_GetActorRotation`)) "Undefined" "OverrideRootScale" null null))
      (`KismetSystemLibrary.PrintString` "Apparition du vent")
      (if (> _returnvalue_x 0.0)
        (set `/Game/Blueprints/WindActor.direction` _returnvalue _returnvalue_2)
        (else
          (set `/Game/Blueprints/WindActor.direction` _returnvalue _returnvalue_2)))
      (set `self.windcharge` 0.0)
      (else
        (`KismetSystemLibrary.PrintString` "Pas assez de charge")))))

(event `self.ReceiveBeginPlay`
  (set `self.PlayerEnume` "NewEnumerator0")
  (bind _returnvalue (`|CreateWidget` "/Game/Blueprints/NewWidgetBlueprint.NewWidgetBlueprint_C"))
  (`UserWidget.AddToViewport` _returnvalue 0)
  (set `self.windcharge` 100.0)
  (set `self.startlocation` (`self.GetTransform`)))

(event `InputAction|Use`
  (params (Key :type "Key Structure"))
  (:`Pressed`
    (`self.use`)))

(event `InputAxis|MoveUp`
  (params (AxisValue :type "Float (single-precision)"))
  (switch `/Game/Blueprints/use/echelle/PlayerDefinedEnume` (`self.PlayerEnume`)
    (:`NewEnumerator2`
      (`self.montée` AxisValue))))

(fn `montée`
  (params (`Axis Value` :type "Float (double-precision)"))
  (`CharacterMovementComponent.SetMovementMode` (`self.CharacterMovement`) "MOVE_None" 0)
  (`self.K2_SetActorLocation` (+ (* (`KismetMathLibrary.MakeVector` 0.0 0.0 20.0) `Axis Value`) (`self.K2_GetActorLocation`)) true))

(fn `UserConstructionScript`)