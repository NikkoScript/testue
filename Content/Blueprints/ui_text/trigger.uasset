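; A trigger actor that spawns a text box in the world the first time something overlaps its collision component.
; The overlap event calls CreateDialogBox, which uses a Spawn flag as a one-shot guard and spawns a Text_box actor at the configured transform.
; It then passes its text, size, material and color variables to the new actor through ChangeText.
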(event `self.CollisionComponent.OnComponentBeginOverlap`
  (params (OverlappedComponent :type "PrimitiveComponent Object Reference") (OtherActor :type "Actor Object Reference") (OtherComp :type "PrimitiveComponent Object Reference") (OtherBodyIndex :type Integer) (bFromSweep :type Boolean) (SweepResult :type "HitResult Structure (by ref)"))
  (`self.Create Dialog Box` (`self.location`) (`self.texte`) (`self.taille`) (`self.material`) (`self.couleur`)))

(fn `Create Dialog Box`
  (params (location :type "Transform Structure") (Text :type String) (Size :type "Float (double-precision)") (Material :type "MaterialInterface Object Reference") (Color :type "Color Structure"))
  (if (not (`self.spawn`))
    (set `self.spawn` true)
    (bind _returnvalue (`|SpawnActorFromClass` "/Game/Blueprints/ui_text/text_box/text_box.text_box_C" location "AlwaysSpawn" "OverrideRootScale" null null))
    (`/Game/Blueprints/ui_text/text_box/text_box.change_text` _returnvalue Text Size Material Color)))

(fn `UserConstructionScript`)