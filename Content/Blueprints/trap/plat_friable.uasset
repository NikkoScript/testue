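; Friable platform trap that starts to fall about a second after something hits it.
; On hit, a delay leads to one of two modes selected by ModePlateforme, both enabling physics simulation on the render component.
; Mode 1 also switches collision to physics-only, while Mode 2 leaves collision unchanged.
; The starting location is saved at BeginPlay but never used, and debug strings print the active mode.
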(event `self.ReceiveBeginPlay`
  (set `self.locationinit` (`SceneComponent.K2_GetComponentLocation` (`self.RenderComponent`))))

(event `self.ReceiveActorBeginOverlap`
  (params (OtherActor :type "Actor Object Reference")))

(event `self.ReceiveTick`
  (params (DeltaSeconds :type "Float (single-precision)")))

(event `self.ReceiveHit`
  (params (MyComp :type "PrimitiveComponent Object Reference") (Other :type "Actor Object Reference") (OtherComp :type "PrimitiveComponent Object Reference") (bSelfMoved :type Boolean) (HitLocation :type "Vector Structure") (HitNormal :type "Vector Structure") (NormalImpulse :type "Vector Structure") (Hit :type "HitResult Structure (by ref)"))
  (`KismetSystemLibrary.Delay` 1.0)
  (if (== (`self.Mode plateforme`) 1)
    (`KismetSystemLibrary.PrintString` "Mode 1")
    (`self.Mode 1`)
    (else
      (`KismetSystemLibrary.PrintString` "Mode 2")
      (`self.Mode 2`))))

(fn `Mode 1`
  (bind _rendercomponent (`self.RenderComponent`))
  (`PrimitiveComponent.SetSimulatePhysics` _rendercomponent true)
  (`PrimitiveComponent.SetCollisionEnabled` _rendercomponent "PhysicsOnly"))

(fn `Mode 2`
  (`PrimitiveComponent.SetSimulatePhysics` (`self.RenderComponent`) true))

(fn `UserConstructionScript`)