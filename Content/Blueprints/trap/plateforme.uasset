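; Blueprint actor for a moving platform trap that travels along a timeline-driven offset from its starting position.
; BeginPlay stores the actor location and waits a configurable start delay before setting a Start flag.
; Once set, Tick plays Timeline_0, whose track, scaled by Coef and added to the stored origin, sets the actor location without sweeping.
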(event `self.ReceiveBeginPlay`
  (set `self.localisationplat` (`self.K2_GetActorLocation`))
  (`KismetSystemLibrary.Delay` (`self.startplat`))
  (set `self.start` true))

(event `self.ReceiveTick`
  (params (DeltaSeconds :type "Float (single-precision)"))
  (if (`self.start`)
    (`|ExecutionSequence`
      (:`then_0`
        (bind (_direction _newtrack_0) (`Timeline|Timeline_0`)
          (:`Update`
            (`self.K2_SetActorLocation` (+ (* _newtrack_0 (`self.coef`)) (`self.localisationplat`)))))))))

(fn `UserConstructionScript`)