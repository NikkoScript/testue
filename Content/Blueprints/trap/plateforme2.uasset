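; A moving platform, filed among the traps, that starts after a configurable delay.
; BeginPlay stores the actor's initial location, waits Startplat2 seconds, then sets the Start2 flag.
; While that flag is set, Tick calls Play on a timeline, whose track is scaled by Coef and added to the stored location to move the actor without sweep.
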(event `self.ReceiveBeginPlay`
  (set `self.localisationplat2` (`self.K2_GetActorLocation`))
  (`KismetSystemLibrary.Delay` (`self.startplat2`))
  (set `self.start2` true))

(event `self.ReceiveTick`
  (params (DeltaSeconds :type "Float (single-precision)"))
  (if (`self.start2`)
    (`|ExecutionSequence`
      (:`then_0`
        (bind (_direction _newtrack_1) (`Timeline|Timeline_1`)
          (:`Update`
            (`self.K2_SetActorLocation` (+ (* _newtrack_1 (`self.coef`)) (`self.localisationplat2`)))))))))

(fn `UserConstructionScript`)