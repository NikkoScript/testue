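; TriggerMsg is a trigger actor that shows a MessageTutorial widget while the PaperCharactertest character is near it.
; On overlap it stores the character, adds the widget to the viewport and sets a Displayed flag that blocks duplicates.
; While displayed, Tick prints the squared distance to the character and removes the widget once a fixed threshold is exceeded, re-arming the trigger.
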(event `self.ReceiveActorBeginOverlap`
  (params (OtherActor :type "Actor Object Reference"))
  (if (not (`self.displayed`))
    (bind _aspaper_charactertest (cast `/Game/Blueprints/PaperCharactertest` OtherActor))
    (set `self.PlayerVariable` _aspaper_charactertest)
    (bind _returnvalue (`|CreateWidget` "/Game/Blueprints/MessageTutorial.MessageTutorial_C"))
    (`UserWidget.AddToViewport` _returnvalue 0)
    (set `self.displayed` true)))

(event `self.ReceiveTick`
  (params (DeltaSeconds :type "Float (single-precision)"))
  (bind _returnvalue (`KismetMathLibrary.VSizeSquared` (- (`self.K2_GetActorLocation`) (`self.K2_GetActorLocation` (`self.PlayerVariable`)))))
  (if (`self.displayed`)
    (`KismetSystemLibrary.PrintString` (`KismetStringLibrary.Conv_DoubleToString` _returnvalue))
    (if (> _returnvalue 50000.0)
      (`Widget.RemoveFromParent` (stale `self.ReceiveActorBeginOverlap` _returnvalue))
      (set `self.displayed` false))))

(fn `UserConstructionScript`)