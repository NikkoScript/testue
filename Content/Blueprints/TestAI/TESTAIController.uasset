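; Test AI controller that drives a PBP_TESTAICharacter around the target points assigned on that pawn.
; On BeginPlay it sets up the BB_TESTAI blackboard, seeds NextPointLocation with the first point's location and runs the BT_TESTAI behavior tree.
; GetNextPoint advances a wrapping index through the pawn's TargetPoints and returns that point's location, giving a looping patrol order.
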(event `self.ReceiveBeginPlay`
  (bind _blackboardcomponent (`self.UseBlackboard` "/Game/Blueprints/TestAI/BB_TESTAI.BB_TESTAI"))
  (`BlackboardComponent.SetValueAsVector` _blackboardcomponent "NextPointLocation" (`self.K2_GetActorLocation` (`|GetArrayItem` (`self.GetTargetPoints`))))
  (`self.RunBehaviorTree` "/Game/Blueprints/TestAI/BT_TESTAI.BT_TESTAI"))

(fn `GetNextPoint`
  (returns (ReturnValue :type "Vector Structure"))
  (bind _targetpoints (`self.GetTargetPoints`))
  (bind _result (`/Engine/EditorBlueprintResources/StandardMacros.IncrementInt` (`self.ActualTargetPointIndex`))
    (:`  `
      (set `self.ActualTargetPointIndex` (mod _result (`KismetArrayLibrary.Array_Length` _targetpoints)))
      (return (`self.K2_GetActorLocation` (`|GetArrayItem` _targetpoints (`self.ActualTargetPointIndex`)))))))

(fn `GetTargetPoints`
  (returns (TargetPoints :type "Array of TargetPoint Object Reference"))
  (bind _aspbp_testaicharacter (cast `/Game/Blueprints/TestAI/PBP_TESTAICharacter` (`self.K2_GetPawn`)))
  (return (`/Game/Blueprints/TestAI/PBP_TESTAICharacter.TargetPoints` _aspbp_testaicharacter)))

(fn `UserConstructionScript`)