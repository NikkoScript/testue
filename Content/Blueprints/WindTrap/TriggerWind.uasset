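; Wind trap trigger actor that fires a linked item's reaction when any actor overlaps it.
; On overlap it calls LinkReaction on LinkedItem, then swaps the active and inactive gem meshes to show the triggered state.
; An Active flag blocks retriggering until a two-second delay resets it and restores the inactive gem.
; A leftover debug "Hello" print runs on every overlap.
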(event `self.ReceiveActorBeginOverlap`
  (params (OtherActor :type "Actor Object Reference"))
  (`KismetSystemLibrary.PrintString` "Hello")
  (if (not (`self.Active`))
    (`/Game/Blueprints/WindTrap/LinkedTrap.LinkReaction` (`self.LinkedItem`))
    (set `self.Active` true)
    (`SceneComponent.SetVisibility` (`self.gemactive`) true false)
    (`SceneComponent.SetVisibility` (`self.geminactive`) false false)
    (`KismetSystemLibrary.Delay` 2.0)
    (set `self.Active` false)
    (`SceneComponent.SetVisibility` (`self.gemactive`) false false)
    (`SceneComponent.SetVisibility` (`self.geminactive`) true false)))

(fn `UserConstructionScript`)