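; RotatingTrap is a wind trap hazard that kills the player character on overlap while its kill zone is active.
; LinkReaction switches the kill zone off, waits a short delay, then switches it back on, opening a temporary safe window.
; Actor overlap runs the parent logic, then calls Deathplayer on any PaperCharactertest if the kill zone is active.
; The graph itself contains no rotation logic.
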(event `self.LinkReaction`
  (set `self.killzoneactiv` false)
  (`KismetSystemLibrary.Delay` 2.0)
  (set `self.killzoneactiv` true))

(event `self.ReceiveActorBeginOverlap`
  (params (OtherActor :type "Actor Object Reference"))
  (`parent.ReceiveActorBeginOverlap` OtherActor)
  (if (`self.killzoneactiv`)
    (bind _aspaper_charactertest (cast `/Game/Blueprints/PaperCharactertest` OtherActor))
    (`/Game/Blueprints/PaperCharactertest.deathplayer` _aspaper_charactertest)))

(fn `UserConstructionScript`
  (`parent.UserConstructionScript`))